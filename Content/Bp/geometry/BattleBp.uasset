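; Battle area actor that spawns a group of minions the first time an actor tagged "player" overlaps it.
; The trigger sets a one-time Visit flag, makes its paper sprite visible beyond the owner, and spawns a randomly sized MinionBp group facing the player.
; Spawn locations come from SetPos, whose random point-within-bounds calculation appears unconnected in the graph.
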(event EventBeginPlay
  (|CallParentFunction)
  (Variables|Default|SetmobNum (Math|Random|RandomIntegerinRange 0 4))
  (bind _returnvalue (Actor|GetActorOfClass "/Game/Bp/player/PlayerBp.PlayerBp_C"))
  (Variables|Default|Setplayer _returnvalue))

(event Collision|EventActorBeginOverlap
  (params (OtherActor :type Actor%20Object%20Reference))
  (if (Actor|ActorHasTag OtherActor "player")
    (if (not (Variables|Default|Getvisit))
      (Variables|Default|Setvisit true)
      (Rendering|SetOnlyOwnerSee (Variables|Default|GetPaperSprite) false :!class /Script/Engine.PrimitiveComponent)
      (for _index (range 0 (Variables|Default|GetmobNum))
        (bind _output_get (Variables|Default|Setpos (Utilities|SetPos)))
        (Game|SpawnActorfromClass "/Game/Bp/enemy/MinionBp.MinionBp_C" (Math|Transform|MakeTransform _output_get (Math|Rotator|FindLookatRotation _output_get (Transformation|GetActorLocation (Variables|Default|Getplayer)))) "AdjustIfPossibleButAlwaysSpawn" 0 0)))))

(fn ConstructionScript
  (|CallParentFunction))