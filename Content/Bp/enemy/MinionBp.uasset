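; Minion enemy Blueprint whose stats scale with the current stage stored in the PlayerData game instance.
; On BeginPlay it derives max HP, starting HP, arm HP as a fraction of max, and attack from the stage number.
; Damage runs the parent logic, then CheckDead clears the blackboard "alive" flag at zero HP and increments the Minion counter in PlayerData.
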(event EventBeginPlay
  (|CallParentFunction)
  (bind _asplayer_data (Utilities|Casting|CastToPlayerData (Game|GetGameInstance)))
  (Utilities|FlowControl|Sequence
    (:then_0
      (bind _output_get (Variables|Default|SetmaxHp (+ 1e+02 (Math|Conversions|ToFloat(Integer) (* (Variables|/Game/Bp/player/PlayerData.PlayerData_C|Getstage _asplayer_data) 10)))))
      (Variables|Default|Sethp _output_get)
      (Variables|Default|SetarmHp (* _output_get 0.2)))
    (:then_1
      (Variables|Default|Setatk (+ 20 (* (Variables|/Game/Bp/player/PlayerData.PlayerData_C|Getstage _asplayer_data) 20))))))

(event Collision|EventActorBeginOverlap
  (params (OtherActor :type Actor%20Object%20Reference))
  (|CallParentFunction OtherActor) ; 지금 이 노드는 비활성 상태입니다. \n핀을 끌어서 다른 노드를 연결하면 활성화됩니다.
)

(event EventTick
  (params (DeltaSeconds :type Float%20%28single-precision%29))
  (|CallParentFunction DeltaSeconds) ; 지금 이 노드는 비활성 상태입니다. \n핀을 끌어서 다른 노드를 연결하면 활성화됩니다.
)

(fn ConstructionScript
  (|CallParentFunction))

(fn Damage
  (|CallParentFunction)
  (CallFunction|CheckDead))

(fn CheckDead
  (if (<= (Variables|Default|Gethp) 0.0)
    (AI|Components|Blackboard|SetValueasBool (AI|GetBlackboard 0) (Utilities|Name|MakeLiteralName "alive") false)
    (bind _asplayer_data (Utilities|Casting|CastToPlayerData (Game|GetGameInstance)))
    (Math|Integer|IncrementInt (Variables|/Game/Bp/player/PlayerData.PlayerData_C|Getminion _asplayer_data))))