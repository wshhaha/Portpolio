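; Exit actor that triggers a boss encounter the first time an actor tagged "player" overlaps it.
; A Visit flag makes the trigger one-shot and the overlap turns off Only Owner See on its paper sprite.
; It then spawns BossBp just above the exit, rotated to look at the PlayerBp actor found in the level.
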(event EventBeginPlay
  (|CallParentFunction) ; 지금 이 노드는 비활성 상태입니다. \n핀을 끌어서 다른 노드를 연결하면 활성화됩니다.
)

(event Collision|EventActorBeginOverlap
  (params (OtherActor :type Actor%20Object%20Reference))
  (bind _returnvalue (Transformation|GetActorLocation))
  (bind _returnvalue_2 (+ _returnvalue "0, 0,100.000000"))
  (if (Actor|ActorHasTag OtherActor "player")
    (if (not (Variables|Default|Getvisit))
      (Variables|Default|Setvisit true)
      (Rendering|SetOnlyOwnerSee (Variables|Default|GetPaperSprite) false :!class /Script/Engine.PrimitiveComponent)
      (bind _returnvalue_3 (Actor|GetActorOfClass "/Game/Bp/player/PlayerBp.PlayerBp_C"))
      (Game|SpawnActorfromClass "/Game/Bp/enemy/BossBp.BossBp_C" (Math|Transform|MakeTransform _returnvalue_2 (Math|Rotator|FindLookatRotation _returnvalue_2 (Transformation|GetActorLocation _returnvalue_3))) "Undefined" 0 0))))

(fn ConstructionScript
  (|CallParentFunction))