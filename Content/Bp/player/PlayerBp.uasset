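; Player character for an archery game, handling movement, sprint, dodge, bow combat, potions and death.
; Tick updates leg and arm stamina, draw tension, speed and HUD, while the PlayerData GameInstance holds health, gold, arrow type and stats.
; Anim Blueprint draw flags gate charging and firing; tension scales arrow velocity, and exhausted arms add random spread and camera shake.
; Taking a hit releases the arrow; death switches to an overhead camera before game over.
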(event EventBeginPlay
  (CallFunction|Init))

(event EventTick
  (params (DeltaSeconds :type Float%20%28single-precision%29))
  (Utilities|FlowControl|Sequence
    (:then_0
      (CallFunction|RestoreStm))
    (:then_1
      (CallFunction|IncreaseTension))
    (:then_2
      (CallFunction|Running))
    (:then_3
      (CallFunction|DecreseArmStamina))
    (:then_4
      (CallFunction|RefreshUI))))

(event Input|ActionEvents|InputActionDodge
  (params (Key :type Key%20Structure :default "None"))
  (:Pressed
    (CallFunction|DoDodge)))

(event Input|ActionEvents|InputActionBuy
  (params (Key :type Key%20Structure :default "None"))
  (:Pressed
    (CallFunction|BuyPotion)))

(event Input|ActionEvents|InputActionUsePotion
  (params (Key :type Key%20Structure :default "None"))
  (:Pressed
    (CallFunction|DrinkPotion)))

(event Input|ActionEvents|InputActionWeapon1
  (params (Key :type Key%20Structure :default "None"))
  (:Pressed
    (Variables|/Game/Bp/player/PlayerData.PlayerData_C|SetarrowState (Variables|Default|Getins) "NewEnumerator0")
    (Appearance|SetBrushfromTexture (Variables|/Game/Bp/player/IngameUI.IngameUI_C|GetarrowImg (Variables|Default|Getui)) "/Game/Asset/mat_texture/long.long" false)))

(event Input|ActionEvents|InputActionWeapon2
  (params (Key :type Key%20Structure :default "None"))
  (:Pressed
    (Variables|/Game/Bp/player/PlayerData.PlayerData_C|SetarrowState (Variables|Default|Getins) "NewEnumerator1")
    (Appearance|SetBrushfromTexture (Variables|/Game/Bp/player/IngameUI.IngameUI_C|GetarrowImg (Variables|Default|Getui)) "/Game/Asset/mat_texture/short.short" false)))

(event Input|ActionEvents|InputActionSprint
  (params (Key :type Key%20Structure :default "None"))
  (:Pressed
    (Variables|Default|Setsprinting true))
  (:Released
    (Variables|Default|Setsprinting false)))

(event Input|ActionEvents|InputActionInfo
  (params (Key :type Key%20Structure :default "None"))
  (bind _ui (Variables|Default|Getui))
  (:Pressed
    (Variables|/Script/Engine.PlayerController|SetbShowMouseCursor (Game|GetPlayerController 0) true)
    (Game|SetGamePaused true)
    (Default|SetStatUI _ui)
    (Widget|SetVisibility (Variables|/Game/Bp/player/IngameUI.IngameUI_C|GetStatWindow _ui) "Visible")))

(event Input|ActionEvents|InputActionFire
  (params (Key :type Key%20Structure :default "None"))
  (bind _anim (Variables|Default|Getanim))
  (:Pressed
    (Variables|Default|SetfireClick true)
    (Variables|/Game/Bp/player/anim/playerAnim.playerAnim_C|Setfire _anim true)
    (Variables|/Game/Bp/player/anim/playerAnim.playerAnim_C|Setrecoil _anim false))
  (:Released
    (CallFunction|Shoot)))

(event Input|AxisEvents|InputAxisTurn
  (params (AxisValue :type Float%20%28single-precision%29))
  (Pawn|Input|AddControllerYawInput AxisValue))

(event Input|AxisEvents|InputAxisLookUp
  (params (AxisValue :type Float%20%28single-precision%29))
  (Pawn|Input|AddControllerPitchInput AxisValue))

(event Input|AxisEvents|InputAxisMoveForward
  (params (AxisValue :type Float%20%28single-precision%29))
  (Pawn|Input|AddMovementInput (Transformation|GetActorForwardVector) AxisValue false))

(event Input|AxisEvents|InputAxisMoveRight
  (params (AxisValue :type Float%20%28single-precision%29))
  (Pawn|Input|AddMovementInput (Transformation|GetActorRightVector) AxisValue false))

(fn ConstructionScript)

(fn DoDodge
  (if (and (not (AI|Components|NavMovement|IsFalling (Variables|Character|GetCharacterMovement))) (>= (Variables|Default|GetlegStamina) 1e+01))
    (bind _dodgedir (CallFunction|SetDodgeDir))
    (Physics|AddImpulse (Variables|Character|GetCharacterMovement) _dodgedir true)
    (Variables|Default|SetlegStamina (- (Variables|Default|GetlegStamina) 1e+01))
    (Audio|PlaySoundatLocation "/Game/Asset/Audio/voice_female_a_effort_jump_action_05_Cue.voice_female_a_effort_jump_action_05_Cue" (Transformation|GetActorLocation) "0, 0, 0" 1.0 1.0 0.0 0 0 0)
    (Variables|/Game/Bp/player/anim/playerAnim.playerAnim_C|Setdodge (Variables|Default|Getanim) true)))

(fn SetDodgeDir
  (if (and (== (Input|AxisValues|GetMoveRight) 0.0) (== (Input|AxisValues|GetMoveForward) 0.0))
    (LocalVariables|Setdir (* (Math|Vector|Normalize (+ (Transformation|GetActorForwardVector) "0,0,0.100000")) 1e+03))
    (else
      (LocalVariables|Setdir (* (Math|Vector|Normalize (+ (* (Transformation|GetActorForwardVector) (Input|AxisValues|GetMoveForward)) (* (Transformation|GetActorRightVector) (Input|AxisValues|GetMoveRight)) "0,0,0.100000")) 1e+03))))
  (return (LocalVariables|Getdir)))

(fn RestoreStm
  (Utilities|FlowControl|Sequence
    (:then_0
      (if (and (== (Input|AxisValues|GetMoveRight) 0.0) (== (Input|AxisValues|GetMoveForward) 0.0))
        (if (>= (Variables|Default|GetlegStamina) (Variables|Default|GetmaxLegStamina))
          (Variables|Default|SetlegStamina (Variables|Default|GetmaxLegStamina))
          (else
            (Variables|Default|SetlegStamina (+ (Variables|Default|GetlegStamina) (* 10 (Utilities|Time|GetWorldDeltaSeconds))))))))
    (:then_1
      (if (not (Variables|/Game/Bp/player/anim/playerAnim.playerAnim_C|GetdrawEnd (Variables|Default|Getanim)))
        (Variables|Default|SetarmStamina (+ (Variables|Default|GetarmStamina) (* 10 (Utilities|Time|GetWorldDeltaSeconds))))
        (if (> (Variables|Default|GetarmStamina) (Variables|Default|GetmaxArmStamina))
          (Variables|Default|SetarmStamina (Variables|Default|GetmaxArmStamina)))))))

(fn IncreaseTension
  (if (Variables|/Game/Bp/player/anim/playerAnim.playerAnim_C|GetdrawOn (Variables|Default|Getanim))
    (if (>= (Variables|Default|Gettension) (Variables|Default|GetmaxTension))
      (Variables|Default|Settension (Variables|Default|GetmaxTension))
      (else
        (Variables|Default|Settension (+ (Variables|Default|Gettension) (* (+ (* (Variables|/Game/Bp/player/PlayerData.PlayerData_C|GetdrawPower (Variables|Default|Getins)) 10) 100) (Utilities|Time|GetWorldDeltaSeconds))))))))

(fn BuyPotion
  (bind _ins (Variables|Default|Getins))
  (if (and (Utilities|IsValid (Variables|Default|GetcurItem)) (>= (Variables|/Game/Bp/player/PlayerData.PlayerData_C|Getgold (Variables|Default|Getins)) 100))
    (bind _result (Math|Integer|IncrementInt (Variables|/Game/Bp/player/PlayerData.PlayerData_C|GetpotionNum (Variables|Default|Getins)))
      (:%20%20
        (Rendering|Components|TextRender|SetText (Variables|/Game/Bp/player/IngameUI.IngameUI_C|GetpotionNum (Variables|Default|Getui)) (Utilities|Text|ToText(Integer) _result false false))
        (Variables|/Game/Bp/player/PlayerData.PlayerData_C|Setgold _ins (- (Variables|/Game/Bp/player/PlayerData.PlayerData_C|Getgold _ins) 100))
        (Default|CallSetGoldUi (Variables|Default|Getins))
        (Actor|DestroyActor (Variables|Default|GetcurItem))
        (Audio|PlaySoundatLocation "/Game/Asset/Audio/buy.buy" (Transformation|GetActorLocation) "0, 0, 0" 1.0 1.0 0.0 0 0 0)))))

(fn AddBuylist
  (params (actor :type Actor%20Object%20Reference))
  (bind _aspotion (Utilities|Casting|CastToPotion actor))
  (Variables|Default|SetcurItem _aspotion)
  (Widget|SetVisibility (Variables|/Game/Bp/player/IngameUI.IngameUI_C|GetShopWindow (Variables|Default|Getui)) "Visible"))

(fn RemoveBuylist
  (Variables|Default|SetcurItem 0)
  (Widget|SetVisibility (Variables|/Game/Bp/player/IngameUI.IngameUI_C|GetShopWindow (Variables|Default|Getui)) "Hidden"))

(fn Init
  (Utilities|FlowControl|Sequence
    (:then_0
      (bind _asplayer_anim (Utilities|Casting|CastToplayerAnim (Components|SkeletalMesh|GetAnimInstance (Variables|Default|GetSkeletalMesh))))
      (Variables|Default|Setanim _asplayer_anim))
    (:then_1
      (bind _asplayer_data (Utilities|Casting|CastToPlayerData (Game|GetGameInstance)))
      (Variables|Default|Setins _asplayer_data))
    (:then_2
      (bind _output_get (Variables|Default|SetmaxLegStamina (Variables|/Game/Bp/player/PlayerData.PlayerData_C|GetmaxLegStamina (Variables|Default|Getins))))
      (Variables|Default|SetlegStamina _output_get))
    (:then_3
      (bind _output_get_2 (Variables|Default|SetmaxArmStamina (Variables|/Game/Bp/player/PlayerData.PlayerData_C|GetmaxArmStamina (Variables|Default|Getins))))
      (Variables|Default|SetarmStamina _output_get_2))
    (:then_4
      (Default|UIInit (Variables|Default|Getui) (Variables|/Game/Bp/player/PlayerData.PlayerData_C|Gethp (Variables|Default|Getins)) (Variables|/Game/Bp/player/PlayerData.PlayerData_C|GetmaxHp (Variables|Default|Getins)) (Variables|/Game/Bp/player/PlayerData.PlayerData_C|GetpotionNum (Variables|Default|Getins)) (Variables|/Game/Bp/player/PlayerData.PlayerData_C|Getgold (Variables|Default|Getins)) (Variables|/Game/Bp/player/PlayerData.PlayerData_C|GetarrowState (Variables|Default|Getins)) (Variables|Default|GetlegStamina) (Variables|/Game/Bp/player/PlayerData.PlayerData_C|GetmaxLegStamina (Variables|Default|Getins)) (Variables|Default|GetarmStamina) (Variables|/Game/Bp/player/PlayerData.PlayerData_C|GetmaxArmStamina (Variables|Default|Getins))))))

(fn DrinkPotion
  (if (and (< (Variables|/Game/Bp/player/PlayerData.PlayerData_C|Gethp (Variables|Default|Getins)) (Variables|/Game/Bp/player/PlayerData.PlayerData_C|GetmaxHp (Variables|Default|Getins))) (> (Variables|/Game/Bp/player/PlayerData.PlayerData_C|GetpotionNum (Variables|Default|Getins)) 0))
    (bind _result (Math|Integer|DecrementInt (Variables|/Game/Bp/player/PlayerData.PlayerData_C|GetpotionNum (Variables|Default|Getins)))
      (:%20%20
        (Rendering|Components|TextRender|SetText (Variables|/Game/Bp/player/IngameUI.IngameUI_C|GetpotionNum (Variables|Default|Getui)) (Utilities|Text|ToText(Integer) _result false false))
        (Variables|/Game/Bp/player/PlayerData.PlayerData_C|Sethp (Variables|Default|Getins) (+ (Variables|/Game/Bp/player/PlayerData.PlayerData_C|Gethp (Variables|Default|Getins)) 10))
        (if (> (Variables|/Game/Bp/player/PlayerData.PlayerData_C|Gethp (Variables|Default|Getins)) (Variables|/Game/Bp/player/PlayerData.PlayerData_C|GetmaxHp (Variables|Default|Getins)))
          (Variables|/Game/Bp/player/PlayerData.PlayerData_C|Sethp (Variables|Default|Getins) (Variables|/Game/Bp/player/PlayerData.PlayerData_C|GetmaxHp (Variables|Default|Getins))))
        (Progress|SetPercent (Variables|/Game/Bp/player/IngameUI.IngameUI_C|GetHpBar (Variables|Default|Getui)) (/ (Math|Conversions|ToFloat(Integer) (Variables|/Game/Bp/player/PlayerData.PlayerData_C|Gethp (Variables|Default|Getins))) (Math|Conversions|ToFloat(Integer) (Variables|/Game/Bp/player/PlayerData.PlayerData_C|GetmaxHp (Variables|Default|Getins)))))
        (CameraFades|StartCameraFade (Game|GetPlayerCameraManager 0) 0.0 0.1 0.2 "(R=0.453125,G=1.000000,B=0.453125,A=1.000000)" false false)
        (Audio|PlaySoundatLocation "/Game/Asset/Audio/heal.heal" (Transformation|GetActorLocation) "0, 0, 0" 1.0 1.0 0.0 0 0 0)))))

(fn ShootShort
  (bind _returnvalue (Game|SpawnActorfromClass "/Game/Bp/player/ShortArrow.ShortArrow_C" (Utilities|SetArrowPos) "AlwaysSpawn" 0 0))
  (Variables|/Game/Bp/player/ArrowBase.ArrowBase_C|Setstate _returnvalue "NewEnumerator1")
  (CallFunction|SetArrowDir (Variables|/Game/Bp/player/ArrowBase.ArrowBase_C|GetProjectileMovement _returnvalue) 50 _returnvalue))

(fn ShootLong
  (bind _returnvalue (Game|SpawnActorfromClass "/Game/Bp/player/LongArrow.LongArrow_C" (Utilities|SetArrowPos) "AlwaysSpawn" 0 0))
  (Variables|/Game/Bp/player/ArrowBase.ArrowBase_C|Setstate _returnvalue "NewEnumerator0")
  (CallFunction|SetArrowDir (Variables|/Game/Bp/player/ArrowBase.ArrowBase_C|GetProjectileMovement _returnvalue) 100 _returnvalue))

(fn Running
  (bind _anim (Variables|Default|Getanim))
  (bind _anim_2 (Variables|Default|Getanim))
  (bind _anim_3 (Variables|Default|Getanim))
  (if (Math|Vector|Equal(Vector) (Math|Vector|MakeVector (Input|AxisValues|GetMoveRight) (Input|AxisValues|GetMoveForward) 0.0) "0, 0, 0" 0.0001)
    (Variables|/Game/Bp/player/anim/playerAnim.playerAnim_C|Setwalk _anim_3 false)
    (Variables|/Game/Bp/player/anim/playerAnim.playerAnim_C|Setrun _anim_3 false)
    (elif (and (Variables|Default|Getsprinting) (> (Variables|Default|GetlegStamina) 0.0))
      (Utilities|FlowControl|Sequence
        (:then_0
          (Variables|/Game/Bp/player/anim/playerAnim.playerAnim_C|Setrun _anim true)
          (Variables|/Game/Bp/player/anim/playerAnim.playerAnim_C|Setwalk _anim false))
        (:then_1
          (if (Variables|Default|GetfireClick)
            (Variables|/Script/Engine.CharacterMovementComponent|SetMaxWalkSpeed (Variables|Character|GetCharacterMovement) 9e+02)
            (Variables|Default|SetlegStamina (- (Variables|Default|GetlegStamina) (* 10 (Utilities|Time|GetWorldDeltaSeconds))))
            (else
              (Variables|/Script/Engine.CharacterMovementComponent|SetMaxWalkSpeed (Variables|Character|GetCharacterMovement) 1.2e+03)
              (Variables|Default|SetlegStamina (- (Variables|Default|GetlegStamina) (* 10 (Utilities|Time|GetWorldDeltaSeconds))))))))
      (else
        (Utilities|FlowControl|Sequence
          (:then_0
            (Variables|/Game/Bp/player/anim/playerAnim.playerAnim_C|Setwalk _anim_2 true)
            (Variables|/Game/Bp/player/anim/playerAnim.playerAnim_C|Setrun _anim_2 false))
          (:then_1
            (if (Variables|Default|GetfireClick)
              (Variables|/Script/Engine.CharacterMovementComponent|SetMaxWalkSpeed (Variables|Character|GetCharacterMovement) 3e+02)
              (else
                (Variables|/Script/Engine.CharacterMovementComponent|SetMaxWalkSpeed (Variables|Character|GetCharacterMovement) 6e+02)))))))))

(fn DecreseArmStamina
  (if (Variables|/Game/Bp/player/anim/playerAnim.playerAnim_C|GetdrawEnd (Variables|Default|Getanim))
    (bind _output_get (Variables|Default|SetarmStamina (- (Variables|Default|GetarmStamina) (* 40 (Utilities|Time|GetWorldDeltaSeconds)))))
    (if (<= _output_get 0.0)
      (Variables|Default|SetarmStamina 0.0)
      (Class|PlayerController|ClientStartCameraShakefromSource (Game|GetPlayerController 0) "/Game/Bp/player/LongAim.LongAim_C"))))

(fn SetArrowDir
  (params (movement :type Movement%20Component%20Object%20Reference) (far :type Integer) (arrow :type Arrow%20Base%20Object%20Reference))
  (if (== 0.0 (Variables|Default|GetarmStamina))
    (bind _output_get (Variables|/Script/Engine.MovementComponent|SetVelocity movement (* (+ (Math|Vector|GetForwardVector (Variables|Default|GetCamera)) (Math|Vector|MakeVector 0.0 (Math|Random|RandomFloatinRange -0.2 0.2) (Math|Random|RandomFloatinRange -0.2 0.2))) (* far (Variables|Default|Gettension)))))
    (Variables|/Game/Bp/player/ArrowBase.ArrowBase_C|Setspeed arrow (Math|Vector|VectorLength _output_get))
    (else
      (bind _output_get_2 (Variables|/Script/Engine.MovementComponent|SetVelocity movement (* (Math|Vector|GetForwardVector (Variables|Default|GetCamera)) (* far (Variables|Default|Gettension)))))
      (Variables|/Game/Bp/player/ArrowBase.ArrowBase_C|Setspeed arrow (Math|Vector|VectorLength _output_get_2)))))

(fn Hit
  (params (damage :type Integer))
  (bind _ins (Variables|Default|Getins))
  (bind _ins_2 (Variables|Default|Getins))
  (Utilities|FlowControl|Sequence
    (:then_0
      (CallFunction|Shoot))
    (:then_1
      (bind _output_get (Variables|/Game/Bp/player/PlayerData.PlayerData_C|Sethp _ins_2 (- (Variables|/Game/Bp/player/PlayerData.PlayerData_C|Gethp _ins_2) damage)))
      (Utilities|FlowControl|Sequence
        (:then_0
          (Progress|SetPercent (Variables|/Game/Bp/player/IngameUI.IngameUI_C|GetHpBar (Variables|Default|Getui)) (/ (Math|Conversions|ToFloat(Integer) (Variables|/Game/Bp/player/PlayerData.PlayerData_C|Gethp _ins)) (Math|Conversions|ToFloat(Integer) (Variables|/Game/Bp/player/PlayerData.PlayerData_C|GetmaxHp _ins)))))
        (:then_1
          (if (<= _output_get 0)
            (if (not (Variables|Default|Getdead))
              (Variables|Default|Setdead true)
              (CallFunction|AfterDead))
            (else
              (Class|PlayerController|ClientStartCameraShakefromSource (Game|GetPlayerController 0) "/Game/Bp/player/HitShake.HitShake_C")
              (Audio|PlaySoundatLocation "/Game/Asset/Audio/voice_female_c_hurt_pain_11_Cue.voice_female_c_hurt_pain_11_Cue" (Transformation|GetActorLocation) "0, 0, 0" 1.0 1.0 0.0 0 0 0))))))))

(fn Shoot
  (bind _returnvalue (Transformation|GetActorLocation))
  (bind _anim (Variables|Default|Getanim))
  (Utilities|FlowControl|Sequence
    (:then_0
      (if (Variables|/Game/Bp/player/anim/playerAnim.playerAnim_C|GetdrawOn (Variables|Default|Getanim))
        (switch Utilities|FlowControl|Switch|SwitchonArrowEnum (Variables|/Game/Bp/player/PlayerData.PlayerData_C|GetarrowState (Variables|Default|Getins))
          (:NewEnumerator0
            (CallFunction|ShootLong))
          (:NewEnumerator1
            (CallFunction|ShootShort)))
        (Audio|PlaySoundatLocation "/Game/Asset/Audio/ArrowSound.ArrowSound" _returnvalue "0, 0, 0" 1.0 1.0 0.0 0 0 0)
        (Class|AISenseHearing|ReportNoiseEvent _returnvalue 1.0 self 0.0 "fire")))
    (:then_1
      (Variables|/Game/Bp/player/anim/playerAnim.playerAnim_C|Setfire _anim false)
      (Variables|/Game/Bp/player/anim/playerAnim.playerAnim_C|SetdrawOn _anim false)
      (Variables|/Game/Bp/player/anim/playerAnim.playerAnim_C|SetdrawEnd _anim false)
      (Variables|Default|Settension 0.0)
      (Variables|Default|SetfireClick false))))

(fn RefreshUI
  (bind _ui (Variables|Default|Getui))
  (bind _tensionbar (Variables|/Game/Bp/player/IngameUI.IngameUI_C|GetTensionBar _ui))
  (Utilities|FlowControl|Sequence
    (:then_0
      (Progress|SetPercent (Variables|/Game/Bp/player/IngameUI.IngameUI_C|GetArmStaminaBar _ui) (/ (Variables|Default|GetarmStamina) (Variables|Default|GetmaxArmStamina))))
    (:then_1
      (Progress|SetPercent (Variables|/Game/Bp/player/IngameUI.IngameUI_C|GetLegStaminaBar _ui) (/ (Variables|Default|GetlegStamina) (Variables|Default|GetmaxLegStamina))))
    (:then_2
      (if (> (Variables|Default|Gettension) 0.0)
        (Widget|SetVisibility _tensionbar "Visible")
        (Progress|SetPercent _tensionbar (/ (Variables|Default|Gettension) (Variables|Default|GetmaxTension)))
        (else
          (Widget|SetVisibility _tensionbar "Hidden"))))))

(fn PlayerDead
  (bind _ins (Variables|Default|Getins))
  (Class|AnimInstance|MontagePause (Variables|Default|Getanim) "/Game/Bp/player/anim/playerMontage.playerMontage")
  (Default|SetGameoverNum (Variables|Default|Getui) (Variables|/Game/Bp/player/PlayerData.PlayerData_C|Getstage _ins) (Variables|/Game/Bp/player/PlayerData.PlayerData_C|Getboss _ins) (Variables|/Game/Bp/player/PlayerData.PlayerData_C|Getminion _ins))
  (Widget|SetVisibility (Variables|/Game/Bp/player/IngameUI.IngameUI_C|GetGameoverWindow (Variables|Default|Getui)) "Visible"))

(fn StageClear
  (bind _returnvalue (Game|GetPlayerController 0))
  (Widget|SetVisibility (Variables|/Game/Bp/player/IngameUI.IngameUI_C|GetStageClearWindow (Variables|Default|Getui)) "Visible")
  (Input|DisableInput _returnvalue)
  (Variables|/Script/Engine.PlayerController|SetbShowMouseCursor _returnvalue true))

(fn SetNewStat
  (bind _ins (Variables|Default|Getins))
  (Utilities|FlowControl|Sequence
    (:then_0
      (Variables|Default|SetmaxLegStamina (Variables|/Game/Bp/player/PlayerData.PlayerData_C|GetmaxLegStamina (Variables|Default|Getins))))
    (:then_1
      (Variables|Default|SetmaxArmStamina (Variables|/Game/Bp/player/PlayerData.PlayerData_C|GetmaxArmStamina (Variables|Default|Getins))))
    (:then_2
      (Default|UIInit (Variables|Default|Getui) (Variables|/Game/Bp/player/PlayerData.PlayerData_C|Gethp _ins) (Variables|/Game/Bp/player/PlayerData.PlayerData_C|GetmaxHp _ins) (Variables|/Game/Bp/player/PlayerData.PlayerData_C|GetpotionNum _ins) (Variables|/Game/Bp/player/PlayerData.PlayerData_C|Getgold _ins) (Variables|/Game/Bp/player/PlayerData.PlayerData_C|GetarrowState _ins) (Variables|Default|GetlegStamina) (Variables|/Game/Bp/player/PlayerData.PlayerData_C|GetmaxLegStamina _ins) (Variables|Default|GetarmStamina) (Variables|/Game/Bp/player/PlayerData.PlayerData_C|GetmaxArmStamina _ins)))))

(fn AfterDead
  (Utilities|FlowControl|Sequence
    (:then_0
      (Audio|PlaySoundatLocation "/Game/Asset/Audio/voice_female_a_death_08_Cue.voice_female_a_death_08_Cue" (Transformation|GetActorLocation) "0, 0, 0" 1.0 1.0 0.0 0 0 0))
    (:then_1
      (Transformation|SetWorldRotation (Variables|Default|GetSkeletalMesh) "0, 0, 0" false false)
      (bind _returnvalue (Actor|GetActorOfClass "/Script/Engine.CameraActor"))
      (Transformation|SetActorTransform _returnvalue (Math|Transform|MakeTransform (+ (Transformation|GetActorLocation) "0, 0,500.000000") "-90.000000,0.0,0.0"))
      (Game|Player|SetViewTargetwithBlend (Game|GetPlayerController 0) _returnvalue 0.0 "VTBlend_Linear" 0.0 true))
    (:then_2
      (bind _returnvalue_2 (Animation|Montage|MontagePlay (Variables|Default|Getanim) "/Game/Bp/player/anim/playerMontage.playerMontage" 1.0 "MontageLength" 0.0 true))
      (Utilities|Time|SetTimerbyFunctionName 0 "PlayerDead" (* _returnvalue_2 0.9))
      (Input|DisableInput (Game|GetPlayerController 0))
      (Variables|/Script/Engine.PlayerController|SetbShowMouseCursor (Game|GetPlayerController 0) true))))