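; StoreBp is a store Blueprint with a paper sprite that reacts the first time the player reaches it.
; On actor overlap it checks for the "player" tag and uses a Visit flag so the response runs only once.
; That first visit turns off Only Owner See on the sprite and spawns a Table actor at the store's location with default rotation and scale.
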(event EventBeginPlay
  (|CallParentFunction) ; 지금 이 노드는 비활성 상태입니다. \n핀을 끌어서 다른 노드를 연결하면 활성화됩니다.
)

(event Collision|EventActorBeginOverlap
  (params (OtherActor :type Actor%20Object%20Reference))
  (if (Actor|ActorHasTag OtherActor "player")
    (if (not (Variables|Default|Getvisit))
      (Variables|Default|Setvisit true)
      (Rendering|SetOnlyOwnerSee (Variables|Default|GetPaperSprite) false :!class /Script/Engine.PrimitiveComponent)
      (Game|SpawnActorfromClass "/Game/Bp/geometry/Table.Table_C" (Math|Transform|MakeTransform (Transformation|GetActorLocation)) "AlwaysSpawn" 0 0))))

(fn ConstructionScript
  (|CallParentFunction))